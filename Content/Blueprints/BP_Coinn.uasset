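; BP_Coinn is a coin pickup that records its collection in the level's save state.
; When BP_ThirdPersonCharacter overlaps the Coin component, it adds itself uniquely to AlteredActors in the GM_SaveLod2 game mode's SGLevelStatee, then destroys itself.
; Its LoadState event calls CollectThyself, which only swaps the coin's material to Glass instead of destroying the actor.
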(event OnComponentBeginOverlap(Coin)
  (params (OverlappedComponent :type Primitive%20Component%20Object%20Reference) (OtherActor :type Actor%20Object%20Reference) (OtherComp :type Primitive%20Component%20Object%20Reference) (OtherBodyIndex :type Integer) (bFromSweep :type Boolean) (SweepResult :type Hit%20Result%20Structure%20%28by%20ref%29))
  ;[0.15 0.15 0.15 0.5] When run into,
  ; was it the player?
  ; if so, find the game mode
  ; add myself to the SG_LevelState savegame array for collected coins
  ; and delete myself.
  (Utilities|Casting|CastToBP_ThirdPersonCharacter OtherActor)
  (bind _asgm_save_lod_2 (Utilities|Casting|CastToGM_SaveLod2 (Game|GetGameMode)))
  (Utilities|Array|AddUnique (Variables|/Game/Blueprints/SavingLoading/SG_LevelStatee.SG_LevelStatee_C|GetAlteredActors (Variables|/Game/Blueprints/SavingLoading/GM_SaveLod2.GM_SaveLod2_C|GetSG_LevelStatee _asgm_save_lod_2)) self)
  (Actor|DestroyActor))

(event Custom|CollectThyself
  (Rendering|Material|SetMaterial (Variables|Default|GetCoin) 0 "/DatasmithContent/Materials/FBXImporter/VRED/Glass.Glass"))

(event EventBeginPlay)

(event Collision|EventActorBeginOverlap
  (params (OtherActor :type Actor%20Object%20Reference)))

(event EventTick
  (params (DeltaSeconds :type Float%20%28single-precision%29)))

(event EventLoadState
  (CallFunction|CollectThyself))

(fn ConstructionScript)