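; BP_ProxMine is a proximity mine that can be picked up, dropped and set off by enemies.
; Pickup attaches it to the mesh's hand_r socket without collision; Drop detaches it and simulates physics for two seconds.
; When a tagged BP_EnemyBase enters the Trigger, a debug-drawn sphere trace gates point damage and a damage event on that enemy alone, then the mine destroys itself.
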(event OnComponentBeginOverlap(Trigger)
  (params (OverlappedComponent :type Primitive%20Component%20Object%20Reference) (OtherActor :type Actor%20Object%20Reference) (OtherComp :type Primitive%20Component%20Object%20Reference) (OtherBodyIndex :type Integer) (bFromSweep :type Boolean) (SweepResult :type Hit%20Result%20Structure%20%28by%20ref%29))
  (bind _mine (Variables|Default|GetMine))
  (bind _returnvalue (Transformation|GetWorldLocation _mine))
  (if (Actor|ActorHasTag OtherActor "Enemy")
    (bind _asbp_enemy_base (Utilities|Casting|CastToBP_EnemyBase OtherActor))
    (Development|PrintString "Prox mine")
    (bind (_outhit _returnvalue_2) (Collision|SphereTraceByChannel _returnvalue _returnvalue 2e+02 "TraceTypeQuery2" false 0 "Persistent"))
    (if _returnvalue_2
      (Development|PrintString "Hit Enemy")
      (Game|Damage|ApplyPointDamage _asbp_enemy_base 1e+02 (.Location (Collision|BreakHitResult _outhit)) _outhit)
      (Class|AISenseDamage|ReportDamageEvent _asbp_enemy_base 0 1e+02 (.Location (Collision|BreakHitResult _outhit)) "0, 0, 0" "None")
      (Actor|DestroyActor))))

(event EventDrop
  (Transformation|DetachFromActor "KeepWorld" "KeepWorld" "KeepRelative")
  (Physics|SetSimulatePhysics (Variables|Default|GetMine) true)
  (Collision|SetCollisionEnabled (Variables|Default|GetMine) "QueryAndPhysics")
  (Utilities|FlowControl|Delay 2.0)
  (Physics|SetSimulatePhysics (Variables|Default|GetMine) false))

(event EventPickup
  (params (SkeletalMesh :type Skeletal%20Mesh%20Component%20Object%20Reference))
  ;[0.15 0.15 0.15 0.5] Pickup Function
  (Development|PrintText (Utilities|Text|FormatText "{name} is getting picked up and attached to {mesh}." (Utilities|String|MakeLiteralString "Machine Gun") SkeletalMesh) true true "(R=1.000000,G=0.000000,B=0.478632,A=1.000000)" 6.0)
  (Transformation|AttachComponentToComponent SkeletalMesh "hand_r" "SnapToTarget" "SnapToTarget" "KeepRelative" true)
  (Collision|SetCollisionEnabled (Variables|Default|GetMine) "NoCollision"))

(fn ConstructionScript)