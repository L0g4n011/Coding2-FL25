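; Shield item Blueprint that a player can pick up, drop or use up, updating that player's HasShield flag.
; Pickup snaps it to the hand_r socket of the given skeletal mesh and disables the Cube's collision.
; Drop detaches it, restores collision, and simulates physics for a short delay before freezing it and clearing the flag.
; UseSecondary destroys the shield and clears the flag.
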(event EventDrop
  (bind _cube (Variables|Default|GetCube))
  (Transformation|DetachFromActor "KeepWorld" "KeepWorld" "KeepRelative")
  (Physics|SetSimulatePhysics _cube true)
  (Collision|SetCollisionEnabled _cube "QueryAndPhysics")
  (Utilities|FlowControl|Delay 2.0)
  (Physics|SetSimulatePhysics _cube false)
  (Variables|/Game/ThirdPerson/Blueprints/BP_ThirdPersonCharacter.BP_ThirdPersonCharacter_C|SetHasShield (stale EventPickup PlayerRef) false))

(event EventPickup
  (params (SkeletalMesh :type Skeletal%20Mesh%20Component%20Object%20Reference) (PlayerRef :type BP%20Third%20Person%20Character%20Object%20Reference))
  ;[0.15 0.15 0.15 0.5] Pickup Function
  (Transformation|AttachComponentToComponent SkeletalMesh "hand_r" "SnapToTarget" "SnapToTarget" "KeepRelative" true)
  (Collision|SetCollisionEnabled (Variables|Default|GetCube) "NoCollision")
  (Variables|/Game/ThirdPerson/Blueprints/BP_ThirdPersonCharacter.BP_ThirdPersonCharacter_C|SetHasShield PlayerRef true))

(event EventUseSecondary
  (Actor|DestroyActor)
  (Variables|/Game/ThirdPerson/Blueprints/BP_ThirdPersonCharacter.BP_ThirdPersonCharacter_C|SetHasShield (stale EventPickup PlayerRef) false))

(fn ConstructionScript)