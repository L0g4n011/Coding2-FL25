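; Keycard item, likely for doors, that the player can pick up, carry and drop.
; Pickup snaps it to the hand_r socket of the supplied skeletal mesh, disables its collision and sets HoldingKeycard on the player.
; Drop detaches it and restores collision with brief physics simulation, freezing it and clearing the flag only after a delay.
; UseSecondary destroys the actor without clearing that flag.
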(event EventBeginPlay)

(event EventDrop
  (Transformation|DetachFromActor "KeepWorld" "KeepWorld" "KeepRelative")
  (Physics|SetSimulatePhysics (Variables|Default|Getkeycard) true)
  (Collision|SetCollisionEnabled (Variables|Default|Getkeycard) "QueryAndPhysics")
  (Utilities|FlowControl|Delay 2.0)
  (Physics|SetSimulatePhysics (Variables|Default|Getkeycard) false)
  (Variables|/Game/ThirdPerson/Blueprints/BP_ThirdPersonCharacter.BP_ThirdPersonCharacter_C|SetHoldingKeycard (stale EventPickup PlayerRef) false))

(event EventTick
  (params (DeltaSeconds :type Float%20%28single-precision%29)))

(event EventPickup
  (params (SkeletalMesh :type Skeletal%20Mesh%20Component%20Object%20Reference) (PlayerRef :type BP%20Third%20Person%20Character%20Object%20Reference))
  (Transformation|AttachComponentToComponent SkeletalMesh "hand_r" "SnapToTarget" "SnapToTarget" "KeepRelative" true)
  (Collision|SetCollisionEnabled (Variables|Default|Getkeycard) "NoCollision")
  (Variables|/Game/ThirdPerson/Blueprints/BP_ThirdPersonCharacter.BP_ThirdPersonCharacter_C|SetHoldingKeycard PlayerRef true))

(event Collision|EventActorBeginOverlap
  (params (OtherActor :type Actor%20Object%20Reference)))

(event EventUseSecondary
  (Actor|DestroyActor))

(fn ConstructionScript)