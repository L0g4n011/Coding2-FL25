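; Fireball projectile that damages an enemy on contact and self-destructs after ten seconds.
; Tick moves it forward a fixed step per frame, without sweep or delta-time scaling.
; The first Trigger overlap with an "Enemy"-tagged actor runs a debug-drawn, single-hit sphere trace on the Camera channel.
; If that hit is a BP_EnemyBase, it applies point damage, reports it to AI damage sensing and destroys itself.
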(event OnComponentBeginOverlap(Trigger)
  (params (OverlappedComponent :type Primitive%20Component%20Object%20Reference) (OtherActor :type Actor%20Object%20Reference) (OtherComp :type Primitive%20Component%20Object%20Reference) (OtherBodyIndex :type Integer) (bFromSweep :type Boolean) (SweepResult :type Hit%20Result%20Structure%20%28by%20ref%29))
  (bind _trigger (Variables|Default|GetTrigger))
  (bind _returnvalue (Transformation|GetWorldLocation _trigger))
  (if (Actor|ActorHasTag OtherActor "Enemy")
    (Utilities|FlowControl|DoOnce false
      (:Completed
        (Development|PrintString "Fireball")
        (bind (_outhit _returnvalue_2) (Collision|SphereTraceByChannel _returnvalue _returnvalue 2e+02 "TraceTypeQuery2" false 0 "Persistent"))
        (if _returnvalue_2
          (bind _asbp_enemy_base (Utilities|Casting|CastToBP_EnemyBase (.HitActor (Collision|BreakHitResult _outhit))))
          (Development|PrintString "Hit Enemy")
          (Game|Damage|ApplyPointDamage _asbp_enemy_base 75.0 (.Location (Collision|BreakHitResult _outhit)) _outhit)
          (Class|AISenseDamage|ReportDamageEvent _asbp_enemy_base 0 75.0 (.Location (Collision|BreakHitResult _outhit)) "0, 0, 0" "None")
          (Actor|DestroyActor))))))

(event EventBeginPlay
  (Utilities|FlowControl|Delay 1e+01)
  (Actor|DestroyActor))

(event Collision|EventActorBeginOverlap
  (params (OtherActor :type Actor%20Object%20Reference)))

(event EventTick
  (params (DeltaSeconds :type Float%20%28single-precision%29))
  (Transformation|SetActorLocation (+ (Transformation|GetActorLocation) (* (Transformation|GetActorForwardVector) 2e+01)) false false))

(fn ConstructionScript)