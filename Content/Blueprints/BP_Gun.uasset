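; BP_Gun is a gun actor that can be picked up and dropped.
; Pickup snaps it to the hand_r socket of the given skeletal mesh and disables the Gun component's collision.
; Drop detaches it in place, restores collision and simulates physics for two seconds before switching simulation off.
; UsePrimary is an empty event with no firing logic.
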(event EventDrop
  (Transformation|DetachFromActor "KeepWorld" "KeepWorld" "KeepRelative")
  (Physics|SetSimulatePhysics (Variables|Default|GetGun) true)
  (Collision|SetCollisionEnabled (Variables|Default|GetGun) "QueryAndPhysics")
  (Utilities|FlowControl|Delay 2.0)
  (Physics|SetSimulatePhysics (Variables|Default|GetGun) false))

(event EventPickup
  (params (SkeletalMesh :type Skeletal%20Mesh%20Component%20Object%20Reference) (PlayerRef :type BP%20Third%20Person%20Character%20Object%20Reference))
  (Transformation|AttachComponentToComponent SkeletalMesh "hand_r" "SnapToTarget" "SnapToTarget" "KeepRelative" true)
  (Collision|SetCollisionEnabled (Variables|Default|GetGun) "NoCollision"))

(event EventUsePrimary)

(fn ConstructionScript)