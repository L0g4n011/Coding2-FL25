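; BP_AiRun is an AI pawn that continuously runs away from the player character.
; It caches the player's BP_ThirdPersonCharacter on BeginPlay and starts the Run event.
; Run projects a point a short step directly away from the player at the pawn's height and moves to a random reachable point around it.
; Run calls itself again whether the move succeeds or fails, so the fleeing loops endlessly.
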(event Custom|Run
  (bind _returnvalue (Transformation|GetActorLocation))
  (bind _player (Variables|Default|GetPlayer))
  (bind _returnvalue_2 (Transformation|GetActorLocation _player))
  (bind _returnvalue_3 (Math|Rotator|FindLookatRotation _returnvalue _returnvalue_2))
  (bind _returnvalue_4 (Math|Vector|GetForwardVector _returnvalue_3))
  (bind _returnvalue_5 (* _returnvalue_4 -1e+02))
  (bind _returnvalue_6 (+ _returnvalue_5 _returnvalue))
  (bind (_x _y) (Math|Vector|BreakVector _returnvalue_6))
  (AI|AIMoveTo self (.RandomLocation (AI|Navigation|GetRandomReachablePointinRadius (Math|Vector|MakeVector _x _y (.Z (Math|Vector|BreakVector _returnvalue))) 2.5e+02 0 0)) 0 5.0 false
    (:OnSuccess
      _)
    (:OnFail
      _))
  (CallFunction|Run))

(event EventBeginPlay
  (bind _asbp_third_person_character (Utilities|Casting|CastToBP_ThirdPersonCharacter (Game|GetPlayerCharacter 0)))
  (Variables|Default|SetPlayer _asbp_third_person_character)
  (CallFunction|Run))

(fn ConstructionScript)