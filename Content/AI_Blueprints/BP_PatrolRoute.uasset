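; Patrol route Blueprint that supplies world-space waypoints along a spline, presumably for AI patrols.
; Each GetPatrolPointLocation call steps PatrolIndex by Direction and returns that spline point's location.
; Direction reverses when the index reaches zero or the point count (one past the last index), producing back-and-forth traversal.
; An unconnected alternative combines both end checks into a single sign flip.
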(fn ConstructionScript)

(fn GetPatrolPointLocation
  (Variables|Default|SetPatrol%20Index (+ (Variables|Default|GetPatrol%20Index) (Variables|Default|GetDirection))) ; go "next" point
  (if (>= (Variables|Default|GetPatrol%20Index) (Spline|GetNumberOfSplinePoints (Variables|Default|GetSpline))) ; are we at the end of the spline?
    (Variables|Default|SetDirection -1) ; reverse the direction
    (elif (<= (Variables|Default|GetPatrol%20Index) 0) ; Are we at the beginning of the spline?
      (Variables|Default|SetDirection 1) ; reverse the direction
    ))
  (return (Spline|GetLocationatSplinePoint (Variables|Default|GetSpline) (Variables|Default|GetPatrol%20Index) "World")))